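; Cartoon waterfall actor that exposes the look of its WaterValley component as tweakable variables.
; The Construction Script creates dynamic materials for slot 0 (opaque or transparent by WaterfallType) and slot 1 (extra foam).
; Two functions push foam, flow, reflection, color and opacity settings into them, plus Day Intensity into the shared MPC_Waterfall collection.
; The EventGraph's duplicate setup and the texture overrides are unconnected and never run.
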(fn `UserConstructionScript`
  (bind _watervalley (`self.WaterValley`))
  (`|ExecutionSequence`
    (:`then_0`
      (bind _returnvalue (`PrimitiveComponent.CreateDynamicMaterialInstance` (`self.WaterValley`) 0 (select `/Game/Shader/Water/Data/WaterfallType` (`self.WaterfallType`) :`NewEnumerator0` "/Game/Shader/Water/Materials/Water/Waterfall/MI_Waterfall_Opaque.MI_Waterfall_Opaque" :`NewEnumerator1` "/Game/Shader/Water/Materials/Water/Waterfall/MI_Waterfall_Transparent.MI_Waterfall_Transparent" :!type "MaterialInterface Object Reference") "None"))
      (bind _output_get (set `self.Instance Mat` _returnvalue))
      (`PrimitiveComponent.SetMaterial` _watervalley 0 _output_get))
    (:`then_1`
      (bind _returnvalue_2 (`PrimitiveComponent.CreateDynamicMaterialInstance` (`self.WaterValley`) 1 "/Game/Shader/Water/Materials/Water/Waterfall/MI_Waterfall_Extra_Foam.MI_Waterfall_Extra_Foam" "None"))
      (bind _output_get_2 (set `self.Extra Instance Mat` _returnvalue_2))
      (`PrimitiveComponent.SetMaterial` _watervalley 1 _output_get_2))
    (:`then_2`
      (`self.Waterfall Parameters`)
      (`self.Waterfall Parameters_Extra`))))

(fn `Waterfall Parameters`
  (bind _instance_mat (`self.Instance Mat`))
  (bind _instance_mat_2 (`self.Instance Mat`))
  (bind _instance_mat_3 (`self.Instance Mat`))
  (bind _instance_mat_4 (`self.Instance Mat`))
  (bind _instance_mat_5 (`self.Instance Mat`))
  (bind _instance_mat_6 (`self.Instance Mat`))
  (`|ExecutionSequence`
    (:`then_0`
      ;[1 1 1] Foam
      (`MaterialInstanceDynamic.SetScalarParameterValue` _instance_mat_4 "Foam Speed" (`self.Foam Speed`))
      (`MaterialInstanceDynamic.SetScalarParameterValue` _instance_mat_4 "Foam X Tile" (`self.Foam X Tile`))
      (`MaterialInstanceDynamic.SetScalarParameterValue` _instance_mat_4 "Foam Y Tile" (`self.Foam Y Tile`))
      (`MaterialInstanceDynamic.SetScalarParameterValue` _instance_mat_4 "Foam Width" (`self.Foam Width`))
      (`MaterialInstanceDynamic.SetScalarParameterValue` _instance_mat_4 "Vertex Offset" (`self.Vertex Offset`))
      (`MaterialInstanceDynamic.SetScalarParameterValue` _instance_mat_4 "Waterfell Flow Speed" (`self.Waterfall Flow Speed`))
      (`KismetMaterialLibrary.SetScalarParameterValue` "/Game/Shader/Water/Materials/MaterialCollections/MPC_Waterfall.MPC_Waterfall" "Day Intensity" (`self.Day Intensity`)))
    (:`then_1`
      ;[1 1 1] Reflection
      (`MaterialInstanceDynamic.SetScalarParameterValue` _instance_mat_6 "Cubemap Intensity" (`self.Cubemap Intensity`))
      (`MaterialInstanceDynamic.SetScalarParameterValue` _instance_mat_6 "Specular Intensity" (`self.Specular Intensity`))
      (`MaterialInstanceDynamic.SetScalarParameterValue` _instance_mat_6 "Reflection Angle" (`self.Reflection Angle`)))
    (:`then_2`
      ;[1 1 1] SSS
      (`MaterialInstanceDynamic.SetScalarParameterValue` _instance_mat_5 "SSS Intensity" (`self.SSS Intensity`))
      (`MaterialInstanceDynamic.SetScalarParameterValue` _instance_mat_5 "SSS Power" (`self.SSS Power`)))
    (:`then_3`
      ;[1 1 1] Normal
      (`MaterialInstanceDynamic.SetScalarParameterValue` _instance_mat_3 "Normal Intensity" (`self.Normal Intensity`))
      (`MaterialInstanceDynamic.SetScalarParameterValue` _instance_mat_3 "Normal X Tile" (`self.Normal X Tile`))
      (`MaterialInstanceDynamic.SetScalarParameterValue` _instance_mat_3 "Normal Y Tile" (`self.Normal Y Tile`))
      (`MaterialInstanceDynamic.SetScalarParameterValue` _instance_mat_3 "Distorsion" (`self.Distorsion`)))
    (:`then_4`
      ;[1 1 1] Color
      (`MaterialInstanceDynamic.SetVectorParameterValue` _instance_mat "Base Color" (`self.Base Color `))
      (`MaterialInstanceDynamic.SetVectorParameterValue` _instance_mat "Far Color" (`self.Specular Color`))
      (`MaterialInstanceDynamic.SetVectorParameterValue` _instance_mat "Foam Color" (`self.Foam Color`))
      (`MaterialInstanceDynamic.SetVectorParameterValue` _instance_mat "SSS Color" (`self.SSS Color`)))
    (:`then_5`
      ;[1 1 1] Opacity
      (`MaterialInstanceDynamic.SetScalarParameterValue` _instance_mat_2 "Opacity" (`self.Opacity`))
      (`MaterialInstanceDynamic.SetScalarParameterValue` _instance_mat_2 "Refraction Normal Intensity" (`self.Refraction Normal Intensity`))
      (`MaterialInstanceDynamic.SetScalarParameterValue` _instance_mat_2 "Refraction" (`self.Refraction`)))))

(fn `Waterfall Parameters_Extra`
  (bind _extra_instance_mat (`self.Extra Instance Mat`))
  (`|ExecutionSequence`
    (:`then_0`
      ;[1 1 1] Foam
      (`MaterialInstanceDynamic.SetScalarParameterValue` _extra_instance_mat "Foam Speed" (`self.Foam Speed`))
      (`MaterialInstanceDynamic.SetScalarParameterValue` _extra_instance_mat "Foam X Tile" (`self.Foam X Tile`))
      (`MaterialInstanceDynamic.SetScalarParameterValue` _extra_instance_mat "Foam Y Tile" (`self.Foam Y Tile`))
      (`MaterialInstanceDynamic.SetScalarParameterValue` _extra_instance_mat "Foam Width" (`self.Foam Width`))
      (`MaterialInstanceDynamic.SetScalarParameterValue` _extra_instance_mat "Vertex Offset" (`self.Vertex Offset`))
      (`MaterialInstanceDynamic.SetScalarParameterValue` _extra_instance_mat "Waterfell Flow Speed" (`self.Waterfall Flow Speed`))
      (`KismetMaterialLibrary.SetScalarParameterValue` "/Game/Shader/Water/Materials/MaterialCollections/MPC_Waterfall.MPC_Waterfall" "Day Intensity" (`self.Day Intensity`)))
    (:`then_1`
      ;[1 1 1] Color
      (`MaterialInstanceDynamic.SetVectorParameterValue` (`self.Extra Instance Mat`) "Foam Color" (`self.Foam Color`)))))
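; BP_FogSheet1 is a fog sheet actor whose look is tuned per instance through exposed variables.
; Its construction script creates a dynamic material instance on the first material slot of StaticMesh1.
; It then copies the variables into that material's parameters, covering color, panning speed, edge softness, fog start fade and depth fade distance.
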(fn `UserConstructionScript`
  (bind _returnvalue (`PrimitiveComponent.CreateDynamicMaterialInstance` (`self.StaticMesh1`) 0 null "None"))
  (`MaterialInstanceDynamic.SetScalarParameterValue` _returnvalue "panningSpeed" (`self.PanningSpeed`))
  (`MaterialInstanceDynamic.SetScalarParameterValue` _returnvalue "SoftEdgesAllAround" (`self.SoftEdgesAllAround`))
  (`MaterialInstanceDynamic.SetVectorParameterValue` _returnvalue "color" (`self.Color`))
  (`MaterialInstanceDynamic.SetScalarParameterValue` _returnvalue "fogStartFadeDistance" (`self.FogStartFadeDistance`))
  (`MaterialInstanceDynamic.SetScalarParameterValue` _returnvalue "DepthfadeDistance" (`self.DepthFadeDistance`)))
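; BP_Comma is the player character Blueprint, handling camera adjustments, a cooldown widget, pausing and load-on-start.
; BeginPlay initializes cooldown tags, caches camera boom defaults, registers itself with the prologue GameInstance and triggers any pending load.
; Activate/Deactivate events set or restore target boom rotation and arm length, which Tick smoothly interpolates toward.
; The pause input lazily creates WBP_Pause and toggles game pause, switching input modes.
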(event `self.ReceiveBeginPlay`
  (bind _gameinstanceref (`self.GameInstanceRef`))
  (bind _aswbp_comma_cooldown (cast `/Game/UI/Widget/Player/WBP_Comma_Cooldown` (`WidgetComponent.GetWidget` (`self.CooldownWidgetComponent`))))
  (`/Game/UI/Widget/Player/WBP_Comma_Cooldown.InitTags` _aswbp_comma_cooldown (`self.CooldownTags`))
  (`|ExecutionSequence`
    (:`then_0`
      (set `self.DefaultCameraRelativeRotation` (`SceneComponent.RelativeRotation` (`self.CameraBoom`)))
      (set `self.TargetCameraRelativeRotation` (`SceneComponent.RelativeRotation` (`self.CameraBoom`)))
      (set `self.DefaultCameraArmLength` (`SpringArmComponent.TargetArmLength` (`self.CameraBoom`)))
      (set `self.TargetCameraArmLength` (`SpringArmComponent.TargetArmLength` (`self.CameraBoom`))))
    (:`then_1`
      (bind _asbp_prologue_game_instance (cast `/Game/SaveGame/BP_PrologueGameInstance` (`GameplayStatics.GetGameInstance`)))
      (bind _output_get (set `self.GameInstanceRef` _asbp_prologue_game_instance))
      (set `/Game/SaveGame/BP_PrologueGameInstance.PlayerCharacter` self _output_get)
      (if (`/Game/SaveGame/BP_PrologueGameInstance.LoadGame?` _gameinstanceref)
        (`/Game/SaveGame/BP_PrologueGameInstance.LoadGame` _gameinstanceref)
        (set `/Game/SaveGame/BP_PrologueGameInstance.LoadGame?` false _gameinstanceref)))))

(event `ActivateRotateCamera`
  (params (NewTargetRotation :type "Rotator Structure"))
  (set `self.TargetCameraRelativeRotation` NewTargetRotation))

(event `self.ReceiveTick`
  (params (DeltaSeconds :type "Float (single-precision)"))
  (`|ExecutionSequence`
    (:`then_0`
      (`SceneComponent.K2_SetRelativeRotation` (`self.CameraBoom`) (`KismetMathLibrary.RInterpTo` (`SceneComponent.RelativeRotation` (`self.CameraBoom`)) (`self.TargetCameraRelativeRotation`) DeltaSeconds (`self.CameraRotationInterpolationSpeed`)) false false))
    (:`then_1`
      (set `SpringArmComponent.TargetArmLength` (`KismetMathLibrary.FInterpTo` (`SpringArmComponent.TargetArmLength` (`self.CameraBoom`)) (`self.TargetCameraArmLength`) DeltaSeconds (`self.CameraArmLengthInterpolationSpeed`)) (`self.CameraBoom`)))))

(event `DeactivateRotateCamera`
  (set `self.TargetCameraRelativeRotation` (`self.DefaultCameraRelativeRotation`)))

(event `ActivateAdjustCamera`
  (params (`New target Arm Length` :type "Float (double-precision)"))
  (set `self.TargetCameraArmLength` `New target Arm Length`))

(event `DeactivateAdjustCamera`
  (set `self.TargetCameraArmLength` (`self.DefaultCameraArmLength`)))

(event `EnhancedInput|/Game/Characters/Comma/Input/Actions/IA_Pause`
  (params (ActionValue :type Boolean) (ElapsedSeconds :type "Float (double-precision)") (TriggeredSeconds :type "Float (double-precision)") (InputAction :type "InputAction Object Reference" :default "/Game/Characters/Comma/Input/Actions/IA_Pause.IA_Pause"))
  (bind _returnvalue (`GameplayStatics.GetPlayerController` 0))
  (bind _pauseref (`self.PauseRef`))
  (:`Started`
    (`/Engine/EditorBlueprintResources/StandardMacros.IsValid` (`self.PauseRef`)
      (:`Is Valid`
        _)
      (:`Is Not Valid`
        (bind _returnvalue_2 (`|CreateWidget` "/Game/UI/Widget/Pause/WBP_Pause.WBP_Pause_C"))
        (set `self.PauseRef` _returnvalue_2)))
    (if (`GameplayStatics.IsGamePaused`)
      (`Widget.RemoveFromParent` (`self.PauseRef`))
      (`GameplayStatics.SetGamePaused` false)
      (`WidgetBlueprintLibrary.SetInputMode_GameOnly` (`GameplayStatics.GetPlayerController` 0))
      (else
        (`UserWidget.AddToViewport` _pauseref 0)
        (`GameplayStatics.SetGamePaused` true)
        (set `PlayerController.bShowMouseCursor` true _returnvalue)
        (`WidgetBlueprintLibrary.SetInputMode_GameAndUIEx` _returnvalue _pauseref)))))

(fn `UserConstructionScript`)
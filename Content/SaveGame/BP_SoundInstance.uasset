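; BP_SoundInstance manages Master, Ambient, Effect and Music volume, backed by a BP_SettingsSave options object.
; After a short delay, Init activates the master sound mix and applies each saved channel value through SetVolume.
; SetVolume clamps values to 0–1, overrides the channel's sound class in the mix, and passes updated options to SetOptions.
; LoadOptions reads the save slot, keeping a newly created object when none exists.
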(event `self.ReceiveInit`
  (bind (_sound_options_master _sound_options_ambient _sound_options_effect _sound_options_music) (break `/Game/SaveGame/SoundOptions` (`/Game/SaveGame/BP_SettingsSave.Sound Options` (`self.SaveOptions`))))
  (`KismetSystemLibrary.Delay` 0.2)
  (`GameplayStatics.SetBaseSoundMix` "/Game/Assets/SFX/SoundClass/MasterSoundClassMix.MasterSoundClassMix")
  (`GameplayStatics.PushSoundMixModifier` "/Game/Assets/SFX/SoundClass/MasterSoundClassMix.MasterSoundClassMix")
  (`self.SaveOptions`
    (:`then`
      _)
    (:`else`
      (`self.LoadOptions`)))
  (`|ExecutionSequence`
    (:`then_0`
      (`self.SetVolume` "NewEnumerator0" _sound_options_master))
    (:`then_1`
      (`self.SetVolume` "NewEnumerator1" _sound_options_ambient))
    (:`then_2`
      (`self.SetVolume` "NewEnumerator2" _sound_options_effect))
    (:`then_3`
      (`self.SetVolume` "NewEnumerator3" _sound_options_music))))

(fn `LoadOptions`
  (bind _returnvalue (`GameplayStatics.DoesSaveGameExist` (`self.SaveOptionsName`)))
  (if (not _returnvalue)
    (`self.SaveOptions`
      (:`then`
        _)
      (:`else`
        (bind _returnvalue_2 (`GameplayStatics.CreateSaveGameObject` "/Game/SaveGame/BP_SettingsSave.BP_SettingsSave_C"))
        (set `self.SaveOptions` _returnvalue_2))))
  (bind _returnvalue_3 (`GameplayStatics.LoadGameFromSlot` (`self.SaveOptionsName`)))
  (bind _asbp_settings_save (cast `/Game/SaveGame/BP_SettingsSave` _returnvalue_3))
  (set `self.SaveOptions` _asbp_settings_save))

(fn `SetVolume`
  (params (SoundChannel :type "/Game/SaveGame/E_SoundChannel Enum" :default "NewEnumerator0") (Value :type "Float (double-precision)"))
  (bind _returnvalue (`KismetMathLibrary.FClamp` Value))
  (`self.SaveOptions`
    (:`then`
      _)
    (:`else`
      (`self.LoadOptions`)))
  (switch `/Game/SaveGame/E_SoundChannel` SoundChannel
    (:`NewEnumerator0`
      ; Set Master Volume
      (`GameplayStatics.SetSoundMixClassOverride` "/Game/Assets/SFX/SoundClass/MasterSoundClassMix.MasterSoundClassMix" "/Game/Assets/SFX/SoundClass/OverAll.OverAll" _returnvalue)
      (bind _structout (setmembers `/Game/SaveGame/SoundOptions` :`StructRef` (`/Game/SaveGame/BP_SettingsSave.Sound Options` (`self.SaveOptions`)) :`Master` _returnvalue))
      (`/Game/SaveGame/BP_SettingsSave.SetOptions` (`self.SaveOptions`) _structout))
    (:`NewEnumerator1`
      ; Set Ambient Volume
      (`GameplayStatics.SetSoundMixClassOverride` "/Game/Assets/SFX/SoundClass/MasterSoundClassMix.MasterSoundClassMix" "/Game/Assets/SFX/SoundClass/MasterAmbient_SoundClass.MasterAmbient_SoundClass" _returnvalue)
      (bind _structout_2 (setmembers `/Game/SaveGame/SoundOptions` :`StructRef` (`/Game/SaveGame/BP_SettingsSave.Sound Options` (`self.SaveOptions`)) :`Ambient` _returnvalue))
      (`/Game/SaveGame/BP_SettingsSave.SetOptions` (`self.SaveOptions`) _structout_2))
    (:`NewEnumerator2`
      ; Set Effects Volume
      (`GameplayStatics.SetSoundMixClassOverride` "/Game/Assets/SFX/SoundClass/MasterSoundClassMix.MasterSoundClassMix" "/Game/Assets/SFX/SoundClass/MasterEffect_SoundClass.MasterEffect_SoundClass" _returnvalue)
      (bind _structout_3 (setmembers `/Game/SaveGame/SoundOptions` :`StructRef` (`/Game/SaveGame/BP_SettingsSave.Sound Options` (`self.SaveOptions`)) :`Effect` _returnvalue))
      (`/Game/SaveGame/BP_SettingsSave.SetOptions` (`self.SaveOptions`) _structout_3))
    (:`NewEnumerator3`
      ; Set Music Volume
      (`GameplayStatics.SetSoundMixClassOverride` "/Game/Assets/SFX/SoundClass/MasterSoundClassMix.MasterSoundClassMix" "/Game/Assets/SFX/SoundClass/MasterMusic_SoundClass.MasterMusic_SoundClass" _returnvalue)
      (bind _structout_4 (setmembers `/Game/SaveGame/SoundOptions` :`StructRef` (`/Game/SaveGame/BP_SettingsSave.Sound Options` (`self.SaveOptions`)) :`Music` _returnvalue))
      (`/Game/SaveGame/BP_SettingsSave.SetOptions` (`self.SaveOptions`) _structout_4))))
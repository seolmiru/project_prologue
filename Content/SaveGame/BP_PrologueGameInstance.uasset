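; Prologue game instance that handles saving and loading player progress through save-game slots.
; SaveGame stores the player's transform, level name and GAS currency attribute, broadcasting save-state changes; LoadGame reapplies transform and currency.
; MenuLoadGame flags a load and opens the level returned by GameLoad, which reads the save slot.
; GameLoad also fetches audio settings, but only when no level name is returned first; trigger functions are empty stubs.
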(event `MenuLoadGame`
  (bind _returnvalue (`GameplayStatics.GetPlayerController` 0))
  (set `self.LoadGame?` true)
  (bind _savedlevel (`self.GameLoad`))
  (`GameplayStatics.OpenLevel` (`KismetStringLibrary.Conv_StringToName` _savedlevel))
  (set `PlayerController.bShowMouseCursor` true _returnvalue)
  (`WidgetBlueprintLibrary.SetInputMode_GameOnly` _returnvalue))

(event `CheckTrigger`)

(fn `GameLoad`
  (returns (SavedLevel :type String))
  (`|ExecutionSequence`
    (:`then_0`
      (bind _returnvalue (`GameplayStatics.LoadGameFromSlot` (`self.SlotNameSave`)))
      (`/Engine/EditorBlueprintResources/StandardMacros.IsValid` _returnvalue
        (:`Is Valid`
          (set `self.bHasSaveData` true)
          (bind _asbp_save_game (cast `/Game/SaveGame/BP_SaveGame` _returnvalue))
          (if (`KismetStringLibrary.IsEmpty` (`PrologueSaveGame.SavedLevelName` (`self.SaveRef`)))
            (set `self.bHasSaveData` false)
            (else
              (bind _output_get (set `self.SaveRef` _asbp_save_game))
              (return (`PrologueSaveGame.SavedLevelName` _output_get)))))
        (:`Is Not Valid`
          (set `self.bHasSaveData` false))))
    (:`then_1`
      (bind _returnvalue_2 (`GameplayStatics.LoadGameFromSlot` "audiosettings"))
      (bind _asbp_settings_save (cast `/Game/SaveGame/BP_SettingsSave` _returnvalue_2))
      (set `self.SavingSettingsRef` _asbp_settings_save))))

(fn `LoadGame`
  (bind _saveref (`self.SaveRef`))
  (`PrologueFunctionLibrary.SetAttributeBaseValue` (`PrologueCharacter.GetAbilitySystemComponent` (`self.PlayerCharacter`)) (struct :`AttributeName` "Currency" :`Attribute` "/Script/Prologue.PrologueSkillAttributeSet:Currency" :`AttributeOwner` "/Script/CoreUObject.Class'/Script/Prologue.PrologueSkillAttributeSet'") (`PrologueSaveGame.SavedCurrency` _saveref))
  (`Actor.K2_SetActorTransform` (`self.PlayerCharacter`) (`/Game/SaveGame/BP_SaveGame.Transform` _saveref) false true))

(fn `LoadTrigger`)

(fn `SaveGame`
  (bind _output_get (set `self.bIsSaving` true))
  (`self.OnSaveStateChanged` _output_get)
  (bind _returnvalue (`GameplayStatics.CreateSaveGameObject` "/Game/SaveGame/BP_SaveGame.BP_SaveGame_C"))
  (bind _output_get_2 (set `self.SaveRef` _returnvalue))
  (set `/Game/SaveGame/BP_SaveGame.Transform` (`Actor.GetTransform` (`self.PlayerCharacter`)) _output_get_2)
  (bind _returnvalue_2 (`GameplayStatics.GetCurrentLevelName` true))
  (set `PrologueSaveGame.SavedLevelName` _returnvalue_2 (`self.SaveRef`))
  (set `PrologueSaveGame.SavedCurrency` (`.ReturnValue` (`AbilitySystemBlueprintLibrary.GetFloatAttributeBaseFromAbilitySystemComponent` (`AbilitySystemBlueprintLibrary.GetAbilitySystemComponent` (`self.PlayerCharacter`)) (struct :`AttributeName` "CurrentHealth" :`Attribute` "/Script/Prologue.PrologueAttributeSet:CurrentHealth" :`AttributeOwner` "/Script/CoreUObject.Class'/Script/Prologue.PrologueAttributeSet'"))) (`self.SaveRef`))
  (`GameplayStatics.SaveGameToSlot` (`self.SaveRef`) (`self.SlotNameSave`))
  (set `self.bHasSaveData` true)
  (bind _output_get_3 (set `self.bIsSaving` false))
  (`self.OnSaveStateChanged` _output_get_3))

(fn `SaveTrigger`)
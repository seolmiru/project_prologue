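; BP_SavePoint is a save point actor that saves the game when BP_Comma overlaps it.
; It caches BP_PrologueGameInstance on BeginPlay, then on overlap sets that instance's save slot name and calls its SaveGame.
; Any overlap adds a WBP_Saving widget before the BP_Comma check, and only the successful save path removes it after a short delay.
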(event `self.ReceiveBeginPlay`
  (bind _asbp_prologue_game_instance (cast `/Game/SaveGame/BP_PrologueGameInstance` (`GameplayStatics.GetGameInstance`)))
  (set `self.PrologueGameInstance` _asbp_prologue_game_instance))

(event `self.ReceiveActorBeginOverlap`
  (params (OtherActor :type "Actor Object Reference"))
  (bind _prologuegameinstance (`self.PrologueGameInstance`))
  (bind _returnvalue (`|CreateWidget` "/Game/UI/Widget/Player/WBP_Saving.WBP_Saving_C"))
  (bind _output_get (set `self.SavingUIRef` _returnvalue))
  (`UserWidget.AddToViewport` _output_get 0)
  (cast `/Game/Characters/Comma/BP_Comma` OtherActor)
  (set `/Game/SaveGame/BP_PrologueGameInstance.SlotNameSave` "savegame" _prologuegameinstance)
  (`/Game/SaveGame/BP_PrologueGameInstance.SaveGame` _prologuegameinstance)
  (`KismetSystemLibrary.Delay` 3.0)
  (`Widget.RemoveFromParent` (`self.SavingUIRef`)))

(fn `UserConstructionScript`)
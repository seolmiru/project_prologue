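; BP_PowerBank is an interactable village power source that opens a linked teleporter to connect the portal.
; When BP_Comma overlaps it before interaction, it sets the guide widget's E-key prompt and enables input on itself.
; The first such overlap also shows a Korean hint in a reaction widget for six seconds.
; Pressing E calls Interact, clears CanInteract and opens the teleporter, with no checks in the key event.
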(event `self.ReceiveActorBeginOverlap`
  (params (OtherActor :type "Actor Object Reference"))
  (if (not (`self.bIsInteracted`))
    (bind _asbp_comma (cast `/Game/Characters/Comma/BP_Comma` OtherActor))
    (bind _aswbp_guide_widget (cast `/Game/UI/Widget/Player/WBP_GuideWidget` (`WidgetComponent.GetWidget` (`Comma.GuideWidgetComponent` _asbp_comma))))
    (set `TextBlock.Text` "Press E to Interact" (`/Game/UI/Widget/Player/WBP_GuideWidget.TextBlock_35` _aswbp_guide_widget))
    (`self.EnableInput` (`GameplayStatics.GetPlayerController` 0))
    (`/Engine/EditorBlueprintResources/StandardMacros.DoOnce` false
      (:`Completed`
        (bind _returnvalue (`|CreateWidget` "/Game/UI/Widget/Player/WBP_ReactionWidget.WBP_ReactionWidget_C" (`GameplayStatics.GetPlayerController` 0)))
        (set `self.ReactionWidgetRef` _returnvalue)
        (set `TextBlock.Text` "마을에 있는 동력원을 작동시켜서 포탈을 연결해야해..." (`/Game/UI/Widget/Player/WBP_ReactionWidget.MinuteHandText` _returnvalue))
        (`UserWidget.AddToViewport` (`self.ReactionWidgetRef`) 0)
        (`KismetSystemLibrary.Delay` 6.0)
        (`Widget.RemoveFromParent` (`self.ReactionWidgetRef`))))))

(event `Key|E`
  (params (Key :type "Key Structure"))
  ;[1 0 0 0.5] Check Before Build
  (:`Pressed`
    (`self.Interact`)
    (set `self.CanInteract` false)
    (`/Game/Assets/BlueprintObjects/BP_Teleporter.OpenTeleporter` (`self.TeleporterRef`))))

(fn `UserConstructionScript`)
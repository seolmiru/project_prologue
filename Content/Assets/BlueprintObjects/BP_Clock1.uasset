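; BP_Clock1 is a clock prop whose second, minute and hour hands rotate continuously.
; Each Tick adds a local pitch rotation to each hand component, using that hand's speed variable scaled by delta seconds for frame-rate independent motion.
; The hands only accumulate rotation over time and never read an actual time value, and the construction script is empty.
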(event `self.ReceiveTick`
  (params (DeltaSeconds :type "Float (single-precision)"))
  (`SceneComponent.K2_AddLocalRotation` (`self.SecondHand`) (`KismetMathLibrary.MakeRotator` 0.0 (* DeltaSeconds (`self.SecondSpeed`))) false false)
  (`SceneComponent.K2_AddLocalRotation` (`self.MinuteHand`) (`KismetMathLibrary.MakeRotator` 0.0 (* (`self.MinuteSpeed`) DeltaSeconds)) false false)
  (`SceneComponent.K2_AddLocalRotation` (`self.HourHand`) (`KismetMathLibrary.MakeRotator` 0.0 (* (`self.HourSpeed`) DeltaSeconds)) false false))

(fn `UserConstructionScript`)